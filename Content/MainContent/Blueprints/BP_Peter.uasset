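; BP_Peter is an animated character actor that plays looping animations on its skeletal mesh.
; On BeginPlay it starts a happy idle loop, and number keys switch it to dance, walk or waving loops.
; Animations are played directly on the mesh component with PlayAnimation, and the construction script is empty.
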(event `self.ReceiveBeginPlay`
  (`SkeletalMeshComponent.PlayAnimation` (`self.SkeletalMesh`) "/Game/MainContent/Art/Animations/Anim_HappyIdle.Anim_HappyIdle" true))

(event `Key|One`
  (params (Key :type "Key Structure"))
  (:`Pressed`
    (`SkeletalMeshComponent.PlayAnimation` (`self.SkeletalMesh`) "/Game/MainContent/Art/Animations/Anim_Gangnam.Anim_Gangnam" true)))

(event `Key|Two`
  (params (Key :type "Key Structure"))
  (:`Pressed`
    (`SkeletalMeshComponent.PlayAnimation` (`self.SkeletalMesh`) "/Game/MainContent/Art/Animations/Anim_Walk.Anim_Walk" true)))

(event `Key|Three`
  (params (Key :type "Key Structure"))
  (:`Pressed`
    (`SkeletalMeshComponent.PlayAnimation` (`self.SkeletalMesh`) "/Game/MainContent/Art/Animations/Anim_Waving.Anim_Waving" true)))

(fn `UserConstructionScript`)